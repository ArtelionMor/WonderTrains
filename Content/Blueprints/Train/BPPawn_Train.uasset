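; Drivable train pawn that the third-person character can board, drive along a rail spline and leave.
; An entry box flags nearby characters as able to enter; possession attaches the player to a socket, and exit detaches, teleports and repossesses them.
; Throttle advances distance along the first Rails actor's spline each frame, unscaled by delta time, snapping position and tangent rotation while spawning explosion particles.
; A timeline-based acceleration branch is never run.
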(event OnComponentBeginOverlap(BoxEntree)
  (params (OverlappedComponent :type Primitive%20Component%20Object%20Reference) (OtherActor :type Actor%20Object%20Reference) (OtherComp :type Primitive%20Component%20Object%20Reference) (OtherBodyIndex :type Integer) (bFromSweep :type Boolean) (SweepResult :type Hit%20Result%20Structure%20%28by%20ref%29))
  (bind _asbp_third_person_character (Utilities|Casting|CastToBP_ThirdPersonCharacter OtherActor))
  (Variables|/Game/ThirdPerson/Blueprints/BP_ThirdPersonCharacter.BP_ThirdPersonCharacter_C|SetVehicule _asbp_third_person_character self)
  (Variables|/Game/ThirdPerson/Blueprints/BP_ThirdPersonCharacter.BP_ThirdPersonCharacter_C|SetCanEnter _asbp_third_person_character true))

(event OnComponentEndOverlap(BoxEntree)
  (params (OverlappedComponent :type Primitive%20Component%20Object%20Reference) (OtherActor :type Actor%20Object%20Reference) (OtherComp :type Primitive%20Component%20Object%20Reference) (OtherBodyIndex :type Integer))
  (bind _asbp_third_person_character (Utilities|Casting|CastToBP_ThirdPersonCharacter OtherActor))
  (Variables|/Game/ThirdPerson/Blueprints/BP_ThirdPersonCharacter.BP_ThirdPersonCharacter_C|SetCanEnter _asbp_third_person_character false))

(event Custom|OnPossessionEvent
  (bind _returnvalue (Transformation|AttachActorToActor (Variables|Default|GetPlayer) self "PlaceholderPlayer" "SnapToTarget" "SnapToTarget" "KeepWorld" true))
  (Variables|Default|SetHave%20A%20Player _returnvalue))

(event EventBeginPlay
  (bind _outactors (Actor|GetAllActorsOfClass "/Game/Blueprints/Train/Rails/Rails.Rails_C"))
  (if (Utilities|Array|IsNotEmpty _outactors)
    (bind _output_get (Variables|Default|SetRefRails (Utilities|Array|Get(acopy) _outactors)))
    (bind _asrails (Utilities|Casting|CastToRails _output_get)
      (:then
        (Variables|Default|SetRefSpline (Utilities|Array|Get(acopy) (Actor|GetComponentsByClass _asrails "/Script/Engine.SplineComponent")))
        (EventDispatchers|BindEventtoOnPossession (delegate Custom|OnPossessionEvent)))
      (:CastFailed
        (Development|PrintString "Cast Failed")))
    (else
      (Development|PrintString "There is no rail in scene"))))

(event Input|ActionEvents|InputActionEnterLeaveTheVehicule
  (params (Key :type Key%20Structure :default "None"))
  (bind _player (Variables|Default|GetPlayer))
  (:Pressed
    (if true
      (Transformation|DetachFromActor (Variables|Default|GetPlayer) "KeepRelative" "KeepRelative" "KeepRelative")
      (Transformation|SetActorTransform _player (Transformation|GetSocketTransform (Variables|Default|GetCombined_2F76DA07) "OutOfTheTrain" "RTS_World") false true)
      (bind _asbp_third_person_character (Utilities|Casting|CastToBP_ThirdPersonCharacter _player))
      (Pawn|Possess (Pawn|GetController) _asbp_third_person_character))))

(event Input|AxisEvents|InputAxisThrotle
  (params (AxisValue :type Float%20%28single-precision%29))
  (bind _refspline (Variables|Default|GetRefSpline))
  (Variables|Default|SetAcceleration AxisValue)
  (bind _output_get (Variables|Default|SetDistance (+ (Variables|Default|GetDistance) (* (Variables|Default|GetAcceleration) 5e+01))))
  (Development|PrintString (Utilities|String|ToString(Float) _output_get))
  (Effects|SpawnEmitteratLocation "/Game/StarterContent/Particles/P_Explosion.P_Explosion" (Spline|GetLocationatDistanceAlongSpline _refspline (Variables|Default|GetDistance) "World"))
  (Transformation|SetActorTransform (Math|Transform|MakeTransform (Spline|GetLocationatDistanceAlongSpline _refspline (Variables|Default|GetDistance) "World") (Math|Conversions|RotationFromXVector (Spline|GetTangentatDistanceAlongSpline _refspline (Variables|Default|GetDistance) "World"))) false true))

(fn ConstructionScript)