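; BP_Train is a drivable train that a third-person character can be flagged to enter.
; Input axes feed throttle, steering and brake straight into the vehicle movement component, while pressing Handbrake sets the handbrake input to false.
; A box overlap hands the train to BP_ThirdPersonCharacter as its Vehicule and sets CanEnter, which is cleared when the overlap ends.
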(event OnComponentBeginOverlap(Box)
  (params (OverlappedComponent :type Primitive%20Component%20Object%20Reference) (OtherActor :type Actor%20Object%20Reference) (OtherComp :type Primitive%20Component%20Object%20Reference) (OtherBodyIndex :type Integer) (bFromSweep :type Boolean) (SweepResult :type Hit%20Result%20Structure%20%28by%20ref%29))
  (bind _asbp_third_person_character (Utilities|Casting|CastToBP_ThirdPersonCharacter OtherActor))
  (Variables|/Game/ThirdPerson/Blueprints/BP_ThirdPersonCharacter.BP_ThirdPersonCharacter_C|SetVehicule _asbp_third_person_character self)
  (Variables|/Game/ThirdPerson/Blueprints/BP_ThirdPersonCharacter.BP_ThirdPersonCharacter_C|SetCanEnter _asbp_third_person_character true))

(event OnComponentEndOverlap(Box)
  (params (OverlappedComponent :type Primitive%20Component%20Object%20Reference) (OtherActor :type Actor%20Object%20Reference) (OtherComp :type Primitive%20Component%20Object%20Reference) (OtherBodyIndex :type Integer))
  (bind _asbp_third_person_character (Utilities|Casting|CastToBP_ThirdPersonCharacter OtherActor))
  (Variables|/Game/ThirdPerson/Blueprints/BP_ThirdPersonCharacter.BP_ThirdPersonCharacter_C|SetCanEnter _asbp_third_person_character false))

(event Input|ActionEvents|InputActionHandbrake
  (params (Key :type Key%20Structure :default "None"))
  (:Pressed
    (Class|ChaosVehicleMovementComponent|SetHandbrakeInput (Variables|Default|GetVehicleMovementComponent) false)))

(event Input|AxisEvents|InputAxisSteerRight
  (params (AxisValue :type Float%20%28single-precision%29))
  (Class|ChaosVehicleMovementComponent|SetSteeringInput (Variables|Default|GetVehicleMovementComponent) AxisValue))

(event Input|AxisEvents|InputAxisThrotle
  (params (AxisValue :type Float%20%28single-precision%29))
  (Class|ChaosVehicleMovementComponent|SetThrottleInput (Variables|Default|GetVehicleMovementComponent) AxisValue))

(event Input|AxisEvents|InputAxisBrake
  (params (AxisValue :type Float%20%28single-precision%29))
  (Class|ChaosVehicleMovementComponent|SetBrakeInput (Variables|Default|GetVehicleMovementComponent) AxisValue))

(fn ConstructionScript)